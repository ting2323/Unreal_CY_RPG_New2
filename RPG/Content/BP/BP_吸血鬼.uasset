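; Player-controlled vampire character that fights BP_殭屍 zombies and collects keys, winning at ten and losing on death.
; Input drives movement, sprint, a montage-timed weapon swap between hand and back, and an alternating two-hit light attack gated by a DoOnce.
; Weapon overlap damages zombies, while capsule overlap collects keys.
; 受傷 reduces health and flags death, which Tick handles once before 遊戲結束 shows the end screen and enables level restart.
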(event `InputAxis|MoveForward` :overrideparent false
  (params (AxisValue :type "Float (single-precision)"))
  ;[1 1 1] 移動
  (if (`self.是否死亡`)
    _
    (elif (`self.能否移動`)
      (`self.AddMovementInput` (`KismetMathLibrary.GetForwardVector` (`KismetMathLibrary.MakeRotator` 0.0 0.0 (.yaw (`self.GetControlRotation`)))) AxisValue))))

(event `InputAxis|MoveRight` :overrideparent false
  (params (AxisValue :type "Float (single-precision)"))
  ;[1 1 1] 移動
  (if (`self.是否死亡`)
    _
    (elif (`self.能否移動`)
      (`self.AddMovementInput` (`KismetMathLibrary.GetRightVector` (`KismetMathLibrary.MakeRotator` 0.0 0.0 (.yaw (`self.GetControlRotation`)))) AxisValue))))

(event `InputAxis|Turn` :overrideparent false
  (params (AxisValue :type "Float (single-precision)"))
  ;[1 1 1] 滑鼠輸入
  (`self.AddControllerYawInput` AxisValue))

(event `InputAxis|LookUp` :overrideparent false
  (params (AxisValue :type "Float (single-precision)"))
  ;[1 1 1] 滑鼠輸入
  (`self.AddControllerPitchInput` AxisValue))

(event `InputAction|衝刺`
  (params (Key :type "Key Structure"))
  (bind _charactermovement (`self.CharacterMovement`))
  ;[1 1 1] 衝刺
  (:`Pressed`
    (set `CharacterMovementComponent.MaxWalkSpeed` 1000.0 _charactermovement) ; 設定最大速度：1000
  )
  (:`Released`
    (set `CharacterMovementComponent.MaxWalkSpeed` 600.0 _charactermovement) ; 設定最大速度：600
  ))

(event `InputAction|切換武器`
  (params (Key :type "Key Structure"))
  (bind `_武器` (`self.武器`))
  ;[1 1 1] 切換武器
  (:`Pressed`
    (if (not (`self.是否死亡`))
      (set `self.是否拿武器` (not (`self.是否拿武器`)))
      (`|PlayMontage` (`self.Mesh`) "/Game/動畫/切換武器_Montage.切換武器_Montage" ; 播放剪輯動畫
        (:`then`
          (if (`self.是否拿武器`)
            (`KismetSystemLibrary.Delay` 0.8) ; 延遲
            (`SceneComponent.K2_AttachToComponent` `_武器` (`self.右手位置`) "None" "KeepRelative" "KeepRelative" "KeepRelative" true) ; 有拿武器：手部
            (else
              (`KismetSystemLibrary.Delay` 0.6)
              (`SceneComponent.K2_AttachToComponent` `_武器` (`self.背部位置`) "None" "KeepWorld" "KeepWorld" "KeepWorld" true) ; 沒拿武器：背部
            ))
          (`KismetSystemLibrary.MoveComponentTo` `_武器`) ; 移動元件到指定位置
        )))))

(event `InputAction|輕攻擊`
  (params (Key :type "Key Structure"))
  ;[1 1 1] 輕攻擊
  (:`Pressed`
    (if (not (`self.是否死亡`))
      (`/Engine/EditorBlueprintResources/StandardMacros.DoOnce` false :!label _label ; 執行一次
        (:`Completed`
          (if (`self.是否拿武器`)
            (`|PlayMontage` (`self.Mesh`) (select `int` (mod (`self.輕攻擊次數`) 2) :`0` "/Game/動畫/輕攻擊第一段_Montage.輕攻擊第一段_Montage" :`1` "/Game/動畫/輕攻擊第二段_Montage.輕攻擊第二段_Montage" :!type "AnimMontage Object Reference") 2.0 ; 播放輕攻擊動畫
              (:`then`
                (`/Engine/EditorBlueprintResources/StandardMacros.IncrementInt` (`self.輕攻擊次數`) ; 遞增：每次加 1
                  (:`  `
                    (`KismetSystemLibrary.Delay` 0.6)
                    (`|ExecutionSequence`
                      (:`then_0`
                        (goto _label :!via `Reset`))
                      (:`then_1`
                        (`KismetSystemLibrary.Delay` 0.8)
                        (set `self.輕攻擊次數` 0)))))))
            (else
              (goto _label :!via `Reset`))))))))

(event `self.ReceiveBeginPlay`
  ;[1 1 1] 添加介面
  (bind _returnvalue (`|CreateWidget` "/Game/BP/BW_介面.BW_介面_C" (`GameplayStatics.GetPlayerController` 0))) ; 建立介面
  (`UserWidget.AddToViewport` _returnvalue 0) ; 添加到畫面上
)

(event `self.武器碰撞區域.OnComponentBeginOverlap`
  (params (OverlappedComponent :type "PrimitiveComponent Object Reference") (OtherActor :type "Actor Object Reference") (OtherComp :type "PrimitiveComponent Object Reference") (OtherBodyIndex :type Integer) (bFromSweep :type Boolean) (SweepResult :type "HitResult Structure (by ref)"))
  (bind `_asbp_殭屍` (cast `/Game/BP/BP_殭屍` OtherActor))
  (`/Game/BP/BP_殭屍.受傷` `_asbp_殭屍` 30.0))

(event `self.CapsuleComponent.OnComponentBeginOverlap`
  (params (OverlappedComponent :type "PrimitiveComponent Object Reference") (OtherActor :type "Actor Object Reference") (OtherComp :type "PrimitiveComponent Object Reference") (OtherBodyIndex :type Integer) (bFromSweep :type Boolean) (SweepResult :type "HitResult Structure (by ref)"))
  (bind `_喇叭` (`self.喇叭`))
  (bind `_asbp_鑰匙` (cast `/Game/BP/BP_鑰匙` OtherActor))
  (`AudioComponent.SetSound` `_喇叭` "/Game/音效/音效_.音效_") ; 設定音效
  (`AudioComponent.Play` `_喇叭` 0.0) ; 播放
  (`self.K2_DestroyActor` `_asbp_鑰匙`)
  (bind _result (`/Engine/EditorBlueprintResources/StandardMacros.IncrementInt` (`self.鑰匙數量`))
    (:`  `
      (if (== _result 10)
        (`self.遊戲結束` 0.5 "恭喜過關！")))))

(event `self.ReceiveTick`
  (params (DeltaSeconds :type "Float (single-precision)"))
  (if (`self.是否死亡`)
    (`/Engine/EditorBlueprintResources/StandardMacros.DoOnce` false ; 執行一次
      (:`Completed`
        (`SkeletalMeshComponent.PlayAnimation` (`self.Mesh`) "/Game/動畫/吸血鬼死亡_Montage.吸血鬼死亡_Montage" false) ; 播放動畫
        (`KismetSystemLibrary.Delay` 3.5) ; 死亡動畫時間
        (`SkeletalMeshComponent.SetPlayRate` (`self.Mesh`) 0.0)
        (`self.遊戲結束` 1.0 "GAME OVER")))))

(event `InputAction|重新遊戲`
  (params (Key :type "Key Structure"))
  ;[1 1 1] 重新遊戲
  (:`Pressed`
    (if (`self.是否遊戲結束`)
      (`GameplayStatics.OpenLevel` "遊戲關卡") ; 開啟地圖
    )))

(fn `UserConstructionScript`)

(fn `切換武器碰撞區域`
  (params (`是否顯示武器碰撞區域` :type Boolean))
  (set `PrimitiveComponent.bGenerateOverlapEvents` `是否顯示武器碰撞區域` (`self.武器碰撞區域`)))

(fn `切換移動`
  (params (`能否移動` :type Boolean))
  (set `self.能否移動` `能否移動`))

(fn `受傷`
  (params (`傷害值` :type "Float (double-precision)"))
  (if (not (`self.是否死亡`))
    (set `self.血量` (- (`self.血量`) `傷害值`))
    (`self.PlayAnimMontage` self "/Game/動畫殭屍/殭屍受傷_Montage.殭屍受傷_Montage" 1.0 "None")
    (if (<= (`self.血量`) 0.0)
      (set `self.是否死亡` true))))